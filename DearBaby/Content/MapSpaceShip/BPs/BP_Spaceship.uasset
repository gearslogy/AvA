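; Player spaceship for the SpaceShip map, moved with Enhanced Input and able to fire projectiles.
; BeginPlay adds the movement mapping context, creates the HUD and sets its points text once from PlayerShipGM's PlayerPoints.
; Two axis actions drive world X/Y movement, while the fire action spawns BP_ShipProjectile with a sound.
; Overlapping an "Enemy"-tagged actor shows the game-over widget, switches to UI input with cursor, and pauses the game.
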(event `self.ReceiveBeginPlay`
  (bind _returnvalue (subsystem `EnhancedInputLocalPlayerSubsystem`))
  (`WidgetBlueprintLibrary.SetInputMode_GameOnly` (`GameplayStatics.GetPlayerController` 0))
  (`KismetSystemLibrary.PrintString` "BP_SpaceShip BeginPlay")
  (`/Engine/EditorBlueprintResources/StandardMacros.IsValid` _returnvalue
    (:`Is Valid`
      (`EnhancedInputSubsystemInterface.AddMappingContext` _returnvalue "/Game/MapSpaceShip/BPs/IMC_Movement.IMC_Movement" 0 (struct))
      (bind _returnvalue_2 (`|CreateWidget` "/Game/MapSpaceShip/BPs/GUI/BP_SpaceShipGUI.BP_SpaceShipGUI_C" (`GameplayStatics.GetPlayerController` 0)))
      (bind _output_get (set `self.GUI` _returnvalue_2))
      (`UserWidget.AddToViewport` _output_get 0)
      (bind _asplayer_ship_gm (cast `/Game/MapSpaceShip/BPs/PlayerShipGM` (`GameplayStatics.GetGameMode`)))
      (`TextBlock.SetText` (`/Game/MapSpaceShip/BPs/GUI/BP_SpaceShipGUI.PointsText` (`self.GUI`)) (`KismetTextLibrary.Conv_StringToText` (`KismetStringLibrary.Concat_StrStr` "Points:" (`KismetStringLibrary.Conv_IntToString` (`/Game/MapSpaceShip/BPs/PlayerShipGM.PlayerPoints` _asplayer_ship_gm))))))))

(event `EnhancedInput|/Game/MapSpaceShip/BPs/IA_WS`
  (params (ActionValue :type "Float (double-precision)") (ElapsedSeconds :type "Float (double-precision)") (TriggeredSeconds :type "Float (double-precision)") (InputAction :type "InputAction Object Reference" :default "/Game/MapSpaceShip/BPs/IA_WS.IA_WS"))
  (:`Triggered`
    (`self.AddMovementInput` (`KismetMathLibrary.MakeVector` 0.0 ActionValue))))

(event `EnhancedInput|/Game/MapSpaceShip/BPs/IA_AD`
  (params (ActionValue :type "Float (double-precision)") (ElapsedSeconds :type "Float (double-precision)") (TriggeredSeconds :type "Float (double-precision)") (InputAction :type "InputAction Object Reference" :default "/Game/MapSpaceShip/BPs/IA_AD.IA_AD"))
  (:`Triggered`
    (`self.AddMovementInput` (`KismetMathLibrary.MakeVector` ActionValue))))

(event `self.ReceiveActorBeginOverlap`
  (params (OtherActor :type "Actor Object Reference"))
  (bind _returnvalue (`GameplayStatics.GetPlayerController` 0))
  (if (`self.ActorHasTag` OtherActor "Enemy")
    (bind _returnvalue_2 (`|CreateWidget` "/Game/MapSpaceShip/BPs/GUI/BP_GameOverGUI.BP_GameOverGUI_C"))
    (`UserWidget.AddToViewport` _returnvalue_2 0)
    (`WidgetBlueprintLibrary.SetInputMode_UIOnlyEx` _returnvalue null)
    (set `PlayerController.bShowMouseCursor` true _returnvalue)
    (`GameplayStatics.SetGamePaused` true)))

(event `EnhancedInput|/Game/MapSpaceShip/BPs/IA_FireProjecttile`
  (params (ActionValue :type Boolean) (ElapsedSeconds :type "Float (double-precision)") (TriggeredSeconds :type "Float (double-precision)") (InputAction :type "InputAction Object Reference" :default "/Game/MapSpaceShip/BPs/IA_FireProjecttile.IA_FireProjecttile"))
  (:`Started`
    (`|SpawnActorFromClass` "/Game/MapSpaceShip/BPs/BP_ShipProjectile.BP_ShipProjectile_C" (`self.GetTransform`) "Undefined" "MultiplyWithRoot" null null)
    (`GameplayStatics.SpawnSoundAtLocation` "/Game/MapSpaceShip/Assets/sounds/TankeFire.TankeFire" (`self.K2_GetActorLocation`) (struct) 1.0 1.0 0.0 null null)))

(fn `UserConstructionScript`)